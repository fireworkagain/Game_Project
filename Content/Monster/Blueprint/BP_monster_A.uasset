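; Side-view monster character that patrols along X between two marker components and watches for the player.
; BeginPlay detaches the markers to fix them in world space; Patrol walks toward a random point between them, re-rolled after random delays.
; Tick stores per-axis player distance and direction, flips the sprite by facing, and prints debug positions.
; Idle patrols until range and height checks pass, then switches to Fllow_Character, which has no behavior here.
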(event Custom|Save_Dis_And_DIr
  (bind _returnvalue (Game|GetPlayerCharacter 0))
  (bind _returnvalue_2 (Transformation|GetActorLocation))
  (bind _returnvalue_3 (Transformation|GetActorLocation _returnvalue))
  (bind _returnvalue_4 (- _returnvalue_3 _returnvalue_2))
  (bind (_x _y _z) (Math|Vector|BreakVector _returnvalue_4))
  (bind _returnvalue_5 (Math|Vector|MakeVector _x 0.0 0.0))
  (bind _returnvalue_6 (Math|Vector|MakeVector 0.0 0.0 _z))
  ;[1 1 1] Dis_And_Dir
  (Variables|Dis_And_Dir|SetDis_X (Math|Vector|VectorLength _returnvalue_5))
  (Variables|DisandDir|SetDis_Z (Math|Vector|VectorLength _returnvalue_6))
  (Variables|DisandDir|SetDir_X (Math|Vector|Normalize _returnvalue_5))
  (Variables|DisandDir|SetDir_Z (Math|Vector|Normalize _returnvalue_6)))

(event Custom|Patrol_Ramdom_point
  ;[1 1 1] Patrol_Random_Point
  (Utilities|FlowControl|Delay (Math|Random|RandomFloatinRange 1.0 5.0))
  (CallFunction|RandomPoint))

(event Custom|Patrol
  (bind _returnvalue (Transformation|GetActorForwardVector))
  ;[1 1 1] Patrol_Move
  (CallFunction|PatrolRamdomPoint)
  (if (|character_location>point1)
    (if (|CollapseGraph)
      (Pawn|Input|AddMovementInput _returnvalue 0.0 false :!label _label)
      (else
        (Pawn|Input|AddMovementInput _returnvalue -1.0 false)))
    (elif (|CollapseGraph_0)
      (goto _label)
      (else
        (Pawn|Input|AddMovementInput _returnvalue 1.0 false)))))

(event Custom|Monster_Rotation
  (bind _sprite (Variables|Default|GetSprite))
  (if (>= (Variables|Patrol|GetRotation) 0.0)
    (Transformation|SetWorldRotation _sprite "0, 0, 0" false false)
    (else
      (Transformation|SetWorldRotation _sprite "0.000000,180.000000,0.000000" false false))))

(event Custom|Monster_Sprite_Rotation
  (if (Class|KismetMathLibrary|NotEqualExactlyVectorVector (Transformation|GetVelocity) "0, 0, 0")
    (if (>= (Variables|Patrol|GetRotation) 0.0)
      (Transformation|SetRelativeLocation (Variables|Default|GetSprite) "3.000000,0.000000,6.000000" false false))))

(event EventTick
  (params (DeltaSeconds :type Float%20%28single-precision%29))
  (CallFunction|SaveDisandDIr)
  (CallFunction|MonsterRotation)
  (Development|PrintString (Utilities|String|ToString(Vector) (Transformation|GetActorLocation)))
  (Development|PrintString (Utilities|String|Append (Utilities|String|ToString(Float) (Variables|Patrol|GetPoint1)) "             :               " (Utilities|String|ToString(Float) (Variables|Patrol|GetPoint2))))
  (switch Utilities|FlowControl|Switch|SwitchonMonster_State (Variables|Default|GetMonster_State)
    (:NewEnumerator0
      (if (and (>= (* (Variables|Patrol|GetRotation) (Variables|Dis_And_Dir|GetDis_X)) 0.0) (<= (* (Variables|Patrol|GetRotation) (Variables|Dis_And_Dir|GetDis_X)) 1.5e+02))
        (if (<= (* (Variables|DisandDir|GetDis_Z) (.Z (Math|Vector|BreakVector (Variables|DisandDir|GetDir_Z)))) 3e+01)
          (Variables|Default|SetMonster_State "NewEnumerator1")
          (else
            (CallFunction|Patrol :!label _label)
            (if (> (.X (Math|Vector|BreakVector (Transformation|GetVelocity))) 0.0)
              (Variables|Patrol|SetRotation 1.0)
              (else
                (Variables|Patrol|SetRotation -1.0)))))
        (else
          (goto _label))))))

(event EventBeginPlay
  (Transformation|DetachFromComponent (Variables|Default|Getpatrol_p1) "KeepWorld" "KeepWorld" "KeepWorld" true)
  (CallFunction|RandomPoint))

(fn ConstructionScript)

(fn RandomPoint
  (bind _patrol_p1 (Variables|Default|Getpatrol_p1))
  (bind _patrol_p2 (Variables|Default|Getpatrol_p2))
  (bind _returnvalue (Transformation|GetWorldLocation _patrol_p1))
  (bind _returnvalue_2 (Transformation|GetWorldLocation _patrol_p2))
  (bind (_x _y _z) (Math|Vector|BreakVector _returnvalue))
  (bind (_x_2 _y_2 _z_2) (Math|Vector|BreakVector _returnvalue_2))
  (if (>= _x _x_2)
    (Variables|Patrol|SetPoint1 (Math|Random|RandomFloatinRange _x _x_2))
    (if (<= _z _z_2)
      (Variables|Patrol|SetPoint2 (Math|Random|RandomFloatinRange _z _z_2))
      (else
        (Variables|Patrol|SetPoint2 (Math|Random|RandomFloatinRange _z_2 _z))))
    (return)
    (else
      (Variables|Patrol|SetPoint1 (Math|Random|RandomFloatinRange _x_2 _x)))))