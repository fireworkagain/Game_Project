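; Player character Blueprint for a 2D side-view shooter with sprinting, dashing, attacks, hold-to-reload, health, knockback, death and respawn.
; Enhanced Input events drive movement and actions, gated by player state, ammo and flags, with animation-instance node jumps playing each action.
; Tick flips the sprite and bullet origin from mouse aim, line-traces for wall cover that selects crouched reloading, and runs reload and dash cooldown.
; Health and stamina regeneration events exist but never run.
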(event Custom|Init_Health
  ;[1 1 1] 체력 기본 설정
  (Variables|Default|SetHP (Variables|Default|GetMaxHP)))

(event Custom|Aiming_Mouse
  (bind _returnvalue (Game|GetPlayerController 0))
  (bind _sprite (Variables|Default|GetSprite))
  (bind _bullet_start_point (Variables|Default|GetBullet_Start_Point))
  (bind _worlddirection (Game|Player|ConvertMouseLocationToWorldSpace _returnvalue))
  (bind (_x _y _z) (Math|Vector|BreakVector _worlddirection))
  ;[1 1 1] 공격 방향 지정
  (Variables|/Script/Engine.PlayerController|SetbShowMouseCursor _returnvalue true)
  (Variables|Default|SetMouse_Rotation_X _x)
  (Variables|Default|SetMouse_Rotation_Z _z)
  (if (> (Variables|Default|GetMouse_Rotation_X) 0.0)
    (Transformation|SetWorldRotation _sprite "0, 0, 0" false false)
    (Transformation|SetRelativeLocation _bullet_start_point "17.000000,0.000000,8.000000" false false)
    (else
      (Transformation|SetWorldRotation _sprite "0.000000,180.000000,0.000000" false false)
      (Transformation|SetRelativeLocation _bullet_start_point "-17.000000,0.000000,8.000000" false false))))

(event Custom|Hold_Reloading
  (bind _animationcomponent (Variables|Default|GetAnimationComponent))
  (bind _animinstance (Variables|/Script/PaperZD.PaperZDAnimationComponent|GetAnimInstance _animationcomponent))
  ;[1 1 1] 재장전
  (if (Variables|Default|GetReloading)
    (Pawn|Components|CharacterMovement|DisableMovement (Variables|Character|GetCharacterMovement))
    (Utilities|FlowControl|Delay 0.6)
    (if (Variables|Default|GetWallHide?)
      (Class|PaperZDAnimInstance|JumptoNode _animinstance "Crouch_Reload" "None")
      (else
        (Class|PaperZDAnimInstance|JumptoNode _animinstance "Reload" "None")))))

(event Custom|Init_Stamina
  ;[1 1 1] 스테미나 기본 설정
  (Variables|Default|SetStamina (Variables|Default|GetMax_Stamina)))

(event Custom|Set_Rotation
  ;[1 1 1] Rotation
  (Variables|Default|SetRotation (Math|Conversions|ToFloat(Boolean) (stale Input|EnhancedActionEvents|EnhancedInputAction ActionValue))))

(event Custom|Death
  ;[1 1 1] 죽음
  (Variables|Default|SetPlayer_State "NewEnumerator2")
  (Class|PaperZDAnimInstance|JumptoNode (Variables|/Script/PaperZD.PaperZDAnimationComponent|GetAnimInstance (Variables|Default|GetAnimationComponent)) "Dead" "New State Machine")
  (Components|Movement|StopMovementImmediately (Variables|Character|GetCharacterMovement))
  (Pawn|Components|CharacterMovement|DisableMovement (Variables|Character|GetCharacterMovement))
  (Utilities|FlowControl|Delay 3.0))

(event Custom|Respawn
  ;[1 1 1] 리스폰
  (Variables|Default|SetPlayer_State "NewEnumerator0")
  (bind _returnvalue (Actor|GetActorOfClass "/Script/Engine.PlayerStart"))
  (Transformation|SetActorLocation (Transformation|GetActorLocation _returnvalue) false false)
  (Pawn|Components|CharacterMovement|SetMovementMode (Variables|Character|GetCharacterMovement) "MOVE_Walking" 0)
  (Class|PaperZDAnimInstance|JumptoNode (Variables|/Script/PaperZD.PaperZDAnimationComponent|GetAnimInstance (Variables|Default|GetAnimationComponent)) "Respawn" "New State Machine"))

(event Custom|Wall_Hide
  (bind _returnvalue (Transformation|GetActorLocation))
  ;[1 1 1] Wall_Hide
  (if (Pawn|Components|CharacterMovement|IsWalking (Variables|Character|GetCharacterMovement))
    (bind _returnvalue_2 (Collision|LineTraceByChannel _returnvalue (+ _returnvalue (* (Transformation|GetActorForwardVector) (* (Variables|Default|GetRotation) 25.0))) "TraceTypeQuery1" false 0 "ForOneFrame"))
    (if _returnvalue_2
      (Variables|Default|SetWallHide? true)
      (else
        (Variables|Default|SetWallHide? false)))))

(event Custom|Dash_Cool
  ;[1 1 1] Dash_Cool_Time
  (Utilities|FlowControl|Delay 0.1)
  (Variables|Default|SetDashCoolTime (Math|Float|Clamp(Float) (- (Variables|Default|GetDashCoolTime) 0.1) 0.0 1.5)))

(event Custom|Heal_Stamina
  ;[1 1 1] 기본 스테미나 회복
  (Utilities|FlowControl|Delay 1.0)
  (Variables|Default|SetStamina (Math|Float|Clamp(Float) (+ (Variables|Default|GetStamina) 1e+01) 0.0 (Variables|Default|GetMax_Stamina))))

(event Custom|Heal_Health
  ;[1 1 1] 기본 체력 회복
  (Utilities|FlowControl|Delay 5.0)
  (Variables|Default|SetHP (Math|Float|Clamp(Float) (+ (Variables|Default|GetHP) 5.0) 0.0 (Variables|Default|GetMaxHP))))

(event Custom|Attack_After
  ;[1 1 1] 공격 이후
  (Utilities|FlowControl|Delay 0.1)
  (Variables|Default|SetPlayer_State "NewEnumerator0"))

(event Custom|Init_BulletCount
  ;[1 1 1] Init_Bullet
  (Variables|Default|SetBullet_Count (Variables|Default|GetBullet_Count_Max)))

(event Input|EnhancedActionEvents|EnhancedInputAction
  (params (ActionValue :type Boolean) (ElapsedSeconds :type Float%20%28double-precision%29) (TriggeredSeconds :type Float%20%28double-precision%29))
  ;[1 1 1] 무브먼트
  (if (not (Variables|Default|GetStand_Attacking))
    (Pawn|Input|AddMovementInput (Transformation|GetActorForwardVector) (Math|Conversions|ToFloat(Boolean) ActionValue) false)))

(event Input|EnhancedActionEvents|EnhancedInputAction
  (params (ActionValue :type Boolean) (ElapsedSeconds :type Float%20%28double-precision%29) (TriggeredSeconds :type Float%20%28double-precision%29))
  ;[1 1 1] 공격
  (if (Math|Boolean|ANDBoolean (Utilities|Enum|NotEqual(Enum) 0 0) (> (Variables|Default|GetBullet_Count) 0) (not (Variables|Default|GetReloading)) (not (Variables|Default|GetRolling)))
    (Variables|Default|SetPlayer_State "NewEnumerator0")
    (if (Utilities|Operators|EqualEqual :A (Transformation|GetVelocity))
      (Class|PaperZDAnimInstance|JumptoNode (Variables|/Script/PaperZD.PaperZDAnimationComponent|GetAnimInstance (Variables|Default|GetAnimationComponent)) "Attack" "None")
      (Variables|Default|SetStand_Attacking true)
      (else
        (Class|PaperZDAnimInstance|JumptoNode (Variables|/Script/PaperZD.PaperZDAnimationComponent|GetAnimInstance (Variables|Default|GetAnimationComponent)) "Running_Attack" "None")))))

(event Input|EnhancedActionEvents|EnhancedInputAction
  (params (ActionValue :type Boolean) (ElapsedSeconds :type Float%20%28double-precision%29) (TriggeredSeconds :type Float%20%28double-precision%29))
  ;[1 1 1] 재장전 트리거
  (:Started
    (if (!= (Variables|Default|GetBullet_Count) (Variables|Default|GetBullet_Count_Max))
      (Variables|Default|SetReloading true)
      (else
        (Variables|Default|SetReloading false :!label _label)
        (Pawn|Components|CharacterMovement|SetMovementMode (Variables|Character|GetCharacterMovement) "MOVE_Walking" 0))))
  (:Canceled
    (goto _label))
  (:Completed
    (goto _label)))

(event Input|EnhancedActionEvents|EnhancedInputAction
  (params (ActionValue :type Boolean) (ElapsedSeconds :type Float%20%28double-precision%29) (TriggeredSeconds :type Float%20%28double-precision%29))
  ;[1 1 1] Sprint
  (:Started
    (CallFunction|StartSprint :!label _label))
  (:Ongoing
    (goto _label))
  (:Canceled
    (CallFunction|EndSprint :!label _label_2))
  (:Completed
    (goto _label_2)))

(event Input|EnhancedActionEvents|EnhancedInputAction
  (params (ActionValue :type Boolean) (ElapsedSeconds :type Float%20%28double-precision%29) (TriggeredSeconds :type Float%20%28double-precision%29))
  ;[1 1 1] Rolling
  (if (Math|Boolean|ANDBoolean (Pawn|Components|CharacterMovement|IsWalking (Variables|Character|GetCharacterMovement)) (Utilities|Enum|Equal(Enum) 0 0) (== (Variables|Default|GetDashCoolTime) 0.0))
    (Variables|Default|SetDashCoolTime 1.5)
    (Character|LaunchCharacter (* (Transformation|GetActorForwardVector) (* (Variables|Default|GetRotation) (Variables|Default|GetDash_STR))) false false)
    (Class|PaperZDAnimInstance|JumptoNode (Variables|/Script/PaperZD.PaperZDAnimationComponent|GetAnimInstance (Variables|Default|GetAnimationComponent)) "Dash" "None")))

(event Game|Damage|EventAnyDamage
  (params (Damage :type Float%20%28single-precision%29) (DamageType :type Damage%20Type%20Object%20Reference) (InstigatedBy :type Controller%20Object%20Reference) (DamageCauser :type Actor%20Object%20Reference))
  ;[1 1 1] 공격을 받으면 다른 행동 정지하고 히트 모션 실행
  (if (and (Utilities|Enum|NotEqual(Enum) (Variables|Default|GetPlayer_State) "NewEnumerator2") (not (Variables|Default|GetRolling)))
    (Variables|Default|SetHP (Math|Float|Clamp(Float) (- (Variables|Default|GetHP) Damage) 0.0 (Variables|Default|GetMaxHP)))
    (if (== (Variables|Default|GetHP) 0.0)
      (CallFunction|Death)
      (else
        (Class|PaperZDAnimInstance|JumptoNode (Variables|/Script/PaperZD.PaperZDAnimationComponent|GetAnimInstance (Variables|Default|GetAnimationComponent)) "Hurt" "New State Machine")
        (Variables|Default|SetPlayer_State "NewEnumerator0")
        (Character|LaunchCharacter (* (Math|Vector|Normalize (Math|Vector|MakeVector (.X (Math|Vector|BreakVector (- (Transformation|GetActorLocation) (Transformation|GetActorLocation DamageCauser)))) 0.0 0.0)) 5e+02) false false)))))

(event EventTick
  (params (DeltaSeconds :type Float%20%28single-precision%29))
  (CallFunction|AimingMouse)
  (CallFunction|SetRotation)
  (CallFunction|WallHide)
  (if (Utilities|Enum|Equal(Enum) (Variables|Default|GetPlayer_State) "NewEnumerator0")
    (CallFunction|HoldReloading)
    (CallFunction|DashCool)))

(event EventBeginPlay
  (bind _asbp_game_controller (Utilities|Casting|CastToBP_GameController (Game|GetPlayerController 0)))
  (Input|AddMappingContext (PlayerController|LocalPlayerSubsystems|GetEnhancedInputLocalPlayerSubsystem _asbp_game_controller) 0 0 "(bIgnoreAllPressedKeysUntilRelease=True,bForceImmediately=False,bNotifyUserSettings=False)")
  (CallFunction|InitHealth)
  (CallFunction|InitStamina)
  (CallFunction|InitBulletCount))

(fn ConstructionScript)

(fn StartSprint
  (bind _charactermovement (Variables|Character|GetCharacterMovement))
  (Variables|/Script/Engine.CharacterMovementComponent|SetMaxWalkSpeed _charactermovement (Math|Float|Clamp(Float) (* (Variables|/Script/Engine.CharacterMovementComponent|GetMaxWalkSpeed _charactermovement) 1.5) 0.0 2.5e+02))
  (Variables|Default|SetSprinting true))

(fn EndSprint
  (Variables|/Script/Engine.CharacterMovementComponent|SetMaxWalkSpeed (Variables|Character|GetCharacterMovement) 1.5e+02)
  (Variables|Default|SetSprinting false))