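; Bullet actor that destroys itself one second after BeginPlay and reports what it hits.
; When its Sphere component begins an overlap, it queries overlapping actors of one object type, ignoring its owner and the player character.
; Each found actor's display name is only printed to screen; no damage or other hit response is applied.
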(event OnComponentBeginOverlap(Sphere)
  (params (OverlappedComponent :type Primitive%20Component%20Object%20Reference) (OtherActor :type Actor%20Object%20Reference) (OtherComp :type Primitive%20Component%20Object%20Reference) (OtherBodyIndex :type Integer) (bFromSweep :type Boolean) (SweepResult :type Hit%20Result%20Structure%20%28by%20ref%29))
  (bind _sphere (Variables|Default|GetSphere))
  (bind _outactors (Collision|ComponentOverlapActors _sphere (Math|Transform|MakeTransform (Transformation|GetWorldLocation _sphere) "0, 0, 0" "1.000000,1.000000,1.000000") (Utilities|Array|MakeArray "ObjectTypeQuery8") 0 (Utilities|Array|MakeArray (Components|GetOwner) (Game|GetPlayerCharacter 0))))
  (for _array_element _outactors
    (Development|PrintString (Utilities|GetDisplayName _array_element))))

(event EventBeginPlay
  (Utilities|FlowControl|Delay 1.0)
  (Actor|DestroyActor))

(fn ConstructionScript)