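; BP_AttackEffect1 is a short-lived player attack hitbox that destroys itself 0.4 seconds after spawning.
; Each Tick snaps its Box to the player BP_Character's AttackStartPoint, then queries overlapping actors of one object type using Arrow1's rotation, ignoring the player.
; Every actor found receives the character's BasicDamage on each tick, with no record of prior hits, so damage repeats throughout the effect's lifetime.
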(event OnComponentBeginOverlap(Box)
  (params (OverlappedComponent :type Primitive%20Component%20Object%20Reference) (OtherActor :type Actor%20Object%20Reference) (OtherComp :type Primitive%20Component%20Object%20Reference) (OtherBodyIndex :type Integer) (bFromSweep :type Boolean) (SweepResult :type Hit%20Result%20Structure%20%28by%20ref%29)))

(event EventBeginPlay
  (Utilities|FlowControl|Delay 0.4)
  (Actor|DestroyActor))

(event Collision|EventActorBeginOverlap
  (params (OtherActor :type Actor%20Object%20Reference)))

(event EventTick
  (params (DeltaSeconds :type Float%20%28single-precision%29))
  (CallFunction|WorldLocation)
  (CallFunction|ApplyDamage))

(fn ConstructionScript)

(fn WorldLocation
  (bind _asbp_character (Utilities|Casting|CastToBP_Character (Game|GetPlayerCharacter 0)))
  (Transformation|SetWorldLocation (Variables|Actor|GetBox) (Transformation|GetWorldLocation (Variables|/Game/New_Project/Blueprint/BP_Charater/BP_Character.BP_Character_C|GetAttack_StartPoint _asbp_character)) false false))

(fn ApplyDamage
  (bind _box (Variables|Actor|GetBox))
  (bind _asbp_character (Utilities|Casting|CastToBP_Character (Game|GetPlayerCharacter 0)))
  (bind _outactors (Collision|ComponentOverlapActors _box (Math|Transform|MakeTransform (Transformation|GetWorldLocation _box) (Transformation|GetWorldRotation (Variables|/Game/New_Project/Blueprint/BP_Charater/BP_Character.BP_Character_C|GetArrow1 _asbp_character)) "1.000000,1.000000,1.000000") (Utilities|Array|MakeArray "ObjectTypeQuery8") 0 (Utilities|Array|MakeArray (Game|GetPlayerCharacter 0))))
  (for _array_element _outactors
    (Game|Damage|ApplyDamage _array_element (Variables|/Game/New_Project/Blueprint/BP_Charater/BP_Character.BP_Character_C|GetBasic_Damage _asbp_character) 0 0)))