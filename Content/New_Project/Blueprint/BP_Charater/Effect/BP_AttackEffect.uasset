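; BP_AttackEffect is a flipbook attack-effect actor that acts as the player character's damage hitbox.
; Each Tick moves the flipbook to BP_Character's AttackStartPoint, then overlaps the Capsule's shape using Arrow1's rotation, filtered to one object type and ignoring the player.
; Every overlapped actor takes the character's BasicDamage on every frame, with no per-target hit tracking.
; The Attack_End event destroys the actor.
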(event Custom|Attack_End
  (Actor|DestroyActor))

(event EventBeginPlay)

(event Collision|EventActorBeginOverlap
  (params (OtherActor :type Actor%20Object%20Reference)))

(event EventTick
  (params (DeltaSeconds :type Float%20%28single-precision%29))
  (CallFunction|WorldLocation)
  (CallFunction|ApplyDamage))

(fn ConstructionScript)

(fn WorldLocation
  (bind _asbp_character (Utilities|Casting|CastToBP_Character (Game|GetPlayerCharacter 0)))
  (Transformation|SetWorldLocation (Variables|Default|GetPaperFlipbook) (Transformation|GetWorldLocation (Variables|/Game/New_Project/Blueprint/BP_Charater/BP_Character.BP_Character_C|GetAttack_StartPoint _asbp_character)) false false))

(fn ApplyDamage
  (bind _capsule (Variables|Default|GetCapsule))
  (bind _asbp_character (Utilities|Casting|CastToBP_Character (Game|GetPlayerCharacter 0)))
  (bind _outactors (Collision|ComponentOverlapActors _capsule (Math|Transform|MakeTransform (Transformation|GetWorldLocation _capsule) (Transformation|GetWorldRotation (Variables|/Game/New_Project/Blueprint/BP_Charater/BP_Character.BP_Character_C|GetArrow1 _asbp_character)) "1.000000,1.000000,1.000000") (Utilities|Array|MakeArray "ObjectTypeQuery8") 0 (Utilities|Array|MakeArray (Game|GetPlayerCharacter 0))))
  (for _array_element _outactors
    (Game|Damage|ApplyDamage _array_element (Variables|/Game/New_Project/Blueprint/BP_Charater/BP_Character.BP_Character_C|GetBasic_Damage _asbp_character) 0 0)))