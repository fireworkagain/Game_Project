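; BP_Bullet is a Monster_A bullet actor with a Cube body, apparently unfinished.
; Its only live logic sets the Cube to a fixed world rotation from Tick after a one-second Delay.
; Functions for overlap damage to BP_Character and for detecting BP_AttackEffect to reflect are never run, and Reflect has no action after its DoOnce.
; A helper returning the player's arrow rotation is also unused.
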(event Collision|EventActorBeginOverlap
  (params (OtherActor :type Actor%20Object%20Reference)))

(event EventTick
  (params (DeltaSeconds :type Float%20%28single-precision%29))
  (Utilities|FlowControl|Delay 1.0)
  (Transformation|SetWorldRotation (Variables|Default|GetCube) "0.000000,180.000000,0.000000" false false))

(fn ConstructionScript)

(fn ApplyDamagetoBPCharacter
  (bind _outactors (Collision|ComponentOverlapActors (Variables|Default|GetCube) (Transformation|GetActorTransform) (Utilities|Array|MakeArray "ObjectTypeQuery3") 0 (Utilities|Array|MakeArray (Components|GetOwner) 0)))
  (for _array_element _outactors
    (Utilities|FlowControl|DoOnce false
      (:Completed
        (bind _asbp_character (Utilities|Casting|CastToBP_Character _array_element))
        (Game|Damage|ApplyDamage _asbp_character (Variables|Default|GetBullet_Damage) 0 (Components|GetOwner))))))

(fn Reflect
  (bind _outactors (Collision|ComponentOverlapActors (Variables|Default|GetCube) (Transformation|GetActorTransform) (Utilities|Array|MakeArray "ObjectTypeQuery7") 0))
  (for _array_element _outactors
    (Utilities|Casting|CastToBP_AttackEffect _array_element)
    (Utilities|FlowControl|DoOnce false)))

(fn Rotation
  (bind _asbp_character (Utilities|Casting|CastToBP_Character (Game|GetPlayerCharacter 0)))
  (bind _output_get (Variables|Default|SetRelative%20Rotation (Variables|/Script/Engine.SceneComponent|GetRelativeRotation (Variables|/Game/New_Project/Blueprint/BP_Charater/BP_Character.BP_Character_C|GetArrow1 _asbp_character))))
  (return _output_get))