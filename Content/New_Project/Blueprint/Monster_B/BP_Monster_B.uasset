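; BP_Monster_B is a side-scrolling sprite enemy that patrols, chases and attacks the player.
; Tick runs a state machine (idle, follow, attack, death), with forward box traces for recognition, aggro and attack range, returning to idle while the player is dead or rolling.
; Idle walks along X toward random points between two detached patrol markers.
; AnyDamage reduces HP, and animation node jumps play attack, hurt and death.
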(event Custom|Save_DIs_Dir
  (bind _returnvalue (Game|GetPlayerCharacter 0))
  (bind _returnvalue_2 (Transformation|GetActorLocation))
  (bind _returnvalue_3 (Transformation|GetActorLocation _returnvalue))
  (bind _returnvalue_4 (- _returnvalue_3 _returnvalue_2))
  (bind (_x _y _z) (Math|Vector|BreakVector _returnvalue_4))
  ;[1 1 1] Save_DIs_And_Dir
  (Variables|Default|SetDistance_X _x)
  (Variables|Default|SetDistance_z _z)
  (Variables|Default|SetDir_X (Math|Vector|Normalize (Math|Vector|MakeVector _x 0.0 0.0)))
  (Variables|Default|SetDir_Z (Math|Vector|Normalize (Math|Vector|MakeVector 0.0 0.0 _z))))

(event Custom|Attack_End
  ;[1 1 1] Attack_End
  (Utilities|FlowControl|Delay 0.8)
  (Pawn|Components|CharacterMovement|SetMovementMode (Variables|Character|GetCharacterMovement) "MOVE_Walking" 0)
  (Variables|Default|SetAttacking false)
  (if (Utilities|Enum|NotEqual(Enum) (Variables|Default|GetMonster_State) "NewEnumerator3")
    (if (CallFunction|AttackRange)
      (Class|BPIHurtStateRequest|HurtStateRequest(Message) (Variables|/Script/PaperZD.PaperZDAnimationComponent|GetAnimInstance (Variables|Default|GetAnimationComponent)) "Attack" "None")
      (else
        (Variables|Default|SetMonster_State "NewEnumerator1")))))

(event Custom|Init_Hp
  ;[1 1 1] Init_HP
  (Variables|Default|SetHP (Variables|Default|GetMax_HP)))

(event Custom|Death
  ;[1 1 1] Death
  (Class|PaperZDAnimInstance|JumptoNode (Variables|/Script/PaperZD.PaperZDAnimationComponent|GetAnimInstance (Variables|Default|GetAnimationComponent)) "Death" "None")
  (Components|Movement|StopMovementImmediately (Variables|Character|GetCharacterMovement))
  (Pawn|Components|CharacterMovement|DisableMovement (Variables|Character|GetCharacterMovement)))

(event Custom|Patrol_Point_delay
  ;[1 1 1] Patrol
  (Utilities|FlowControl|Delay (Math|Random|RandomFloatinRange 1.0 5.0))
  (CallFunction|RandomPatrolPoint))

(event Game|Damage|EventAnyDamage
  (params (Damage :type Float%20%28single-precision%29) (DamageType :type Damage%20Type%20Object%20Reference) (InstigatedBy :type Controller%20Object%20Reference) (DamageCauser :type Actor%20Object%20Reference))
  ;[1 1 1] Any_Damage
  (if (Utilities|Enum|NotEqual(Enum) (Variables|Default|GetMonster_State) "NewEnumerator3")
    (Variables|Default|SetBattle false)
    (Variables|Default|SetHP (Math|Float|Clamp(Float) (- (Variables|Default|GetHP) Damage) 0.0 (Variables|Default|GetMax_HP)))
    (if (<= (Variables|Default|GetHP) 0.0)
      (Variables|Default|SetMonster_State "NewEnumerator3")
      (else
        (Class|PaperZDAnimInstance|JumptoNode (Variables|/Script/PaperZD.PaperZDAnimationComponent|GetAnimInstance (Variables|Default|GetAnimationComponent)) "Hurt" "None")))))

(event EventTick
  (params (DeltaSeconds :type Float%20%28single-precision%29))
  ;[1 1 1] AI
  (Development|PrintString (Utilities|String|EnumtoString (Variables|Default|GetMonster_State)))
  (CallFunction|SaveDIsDir)
  (CallFunction|SpriteRotation)
  (CallFunction|NewFunction)
  (switch Utilities|FlowControl|Switch|SwitchonMonster_State (Variables|Default|GetMonster_State)
    (:NewEnumerator0
      (Variables|Default|SetBattle false)
      (CallFunction|PatrolMove)
      (CallFunction|RecongnitionRange))
    (:NewEnumerator1
      (if (CallFunction|AggroRange)
        (if (CallFunction|AttackRange)
          (Variables|Default|SetMonster_State "NewEnumerator2")
          (Variables|Default|SetAttacking true)
          (Class|PaperZDAnimInstance|JumptoNode (Variables|/Script/PaperZD.PaperZDAnimationComponent|GetAnimInstance (Variables|Default|GetAnimationComponent)) "Attack" "None")
          (Pawn|Components|CharacterMovement|DisableMovement (Variables|Character|GetCharacterMovement))
          (else
            (Pawn|Input|AddMovementInput (Variables|Default|GetDir_X) 1.0 false)
            (if (> (.X (Math|Vector|BreakVector (Variables|Default|GetDir_X))) 0.0)
              (Variables|Default|SetRotation 1.0)
              (else
                (Variables|Default|SetRotation -1.0)))))
        (else
          (Variables|Default|SetMonster_State "NewEnumerator0"))))
    (:NewEnumerator2
      (if (not (Variables|Default|GetAttacking))
        (if (not (CallFunction|AttackRange))
          (Variables|Default|SetMonster_State "NewEnumerator1"))))
    (:NewEnumerator3
      (Utilities|FlowControl|DoOnce false
        (:Completed
          (CallFunction|Death))))))

(event EventBeginPlay
  (Transformation|DetachFromComponent (Variables|Default|GetPatrol-point_1) "KeepWorld" "KeepWorld" "KeepWorld" true)
  (CallFunction|InitHp))

(fn ConstructionScript)

(fn RandomPatrolPoint
  (bind _patrol_point_2 (Variables|Default|GetPatrol-point_2))
  (bind _patrol_point_1 (Variables|Default|GetPatrol-point_1))
  (bind _returnvalue (Transformation|GetWorldLocation _patrol_point_1))
  (bind _returnvalue_2 (Transformation|GetWorldLocation _patrol_point_2))
  (bind (_x _y _z) (Math|Vector|BreakVector _returnvalue_2))
  (bind (_x_2 _y_2 _z_2) (Math|Vector|BreakVector _returnvalue))
  (if (<= _x _x_2)
    (Variables|Default|SetPoint_X (Math|Random|RandomFloatinRange _x _x_2))
    (else
      (Variables|Default|SetPoint_X (Math|Random|RandomFloatinRange _x_2 _x))))
  (if (<= _z _z_2)
    (Variables|Default|SetPoint_Z (Math|Random|RandomFloatinRange _z _z_2))
    (else
      (Variables|Default|SetPoint_Z (Math|Random|RandomFloatinRange _z_2 _z)))))

(fn PatrolMove
  (bind _returnvalue (Transformation|GetActorLocation))
  (bind _returnvalue_2 (Transformation|GetActorLocation))
  (bind _point_x (Variables|Default|GetPoint_X))
  (bind _point_x_2 (Variables|Default|GetPoint_X))
  (bind _x (Math|Vector|BreakVector _returnvalue))
  (bind _x_2 (Math|Vector|BreakVector _returnvalue_2))
  (bind _returnvalue_3 (- _x _point_x_2))
  (bind _returnvalue_4 (- _x_2 _point_x))
  (CallFunction|PatrolPointDelay)
  (if (not (and (<= _returnvalue_4 0.1) (>= _returnvalue_4 -0.1)))
    (if (not (and (<= _returnvalue_3 1.0) (>= _returnvalue_3 -1.0)))
      (if (> (.X (Math|Vector|BreakVector (Transformation|GetActorLocation))) (Variables|Default|GetPoint_X))
        (Pawn|Input|AddMovementInput "1.000000,0.000000,0.000000" -1.0 false)
        (Variables|Default|SetRotation -1.0)
        (else
          (Pawn|Input|AddMovementInput "1.000000,0.000000,0.000000" 1.0 false)
          (Variables|Default|SetRotation 1.0))))))

(fn SpriteRotation
  (bind _returnvalue (Transformation|GetVelocity))
  (bind _sprite (Variables|Default|GetSprite))
  (bind _x (Math|Vector|BreakVector _returnvalue))
  (if (> _x 0.0)
    (Transformation|SetRelativeRotation _sprite "0, 0, 0" false false)
    (elif (< _x 0.0)
      (Transformation|SetRelativeRotation _sprite "0.000000,180.000000,0.000000" false false))))

(fn RecongnitionRange
  (Variables|Default|SetRange_Value 1e+02)
  (bind _outhits (Class|KismetSystemLibrary|BoxTraceMultiforObjects (Transformation|GetActorLocation) "0, 0, 0" (Math|Vector|MakeVector 8e+01 5.0 16.0) (Math|Rotator|MakeRotator (Variables|Default|GetRotation) 0.0 0.0) (Utilities|Array|MakeArray "ObjectTypeQuery3") false (Utilities|Array|MakeArray (Components|GetOwner)) "None" true "(R=1.000000,G=0.000000,B=0.000000,A=1.000000)" "(R=0.000000,G=1.000000,B=0.000000,A=1.000000)" 1.0))
  (for _array_element _outhits
    (Utilities|Casting|CastToBP_Character (.HitActor (Collision|BreakHitResult _array_element)))
    (Variables|Default|SetMonster_State "NewEnumerator1")))

(fn DrawDebugBox
  (Rendering|Debug|DrawDebugBox (Transformation|GetActorLocation) "180.000000,20.000000,20.000000" "(R=1.000000,G=0.000000,B=0.010241,A=1.000000)" "0.000000,0.000000,1.000000" 1.0 1.0))

(fn AggroRange
  (bind _returnvalue (Transformation|GetActorLocation))
  (Variables|Default|SetRange_Value 2.8e+02)
  (bind (_outhits _returnvalue_2) (Class|KismetSystemLibrary|BoxTraceMultiforObjects _returnvalue (+ _returnvalue (Math|Vector|MakeVector (* (Variables|Default|GetRotation) (Variables|Default|GetRange_Value)) 0.0 0.0)) (Math|Vector|MakeVector 8e+01 5.0 16.0) (Math|Rotator|MakeRotator (Variables|Default|GetRotation) 0.0 0.0) (Utilities|Array|MakeArray "ObjectTypeQuery3") false (Utilities|Array|MakeArray (Components|GetOwner)) "None" true "(R=1.000000,G=0.000000,B=0.000000,A=1.000000)" "(R=0.000000,G=1.000000,B=0.000000,A=1.000000)" 1.0))
  (for _array_element _outhits
    (Utilities|Casting|CastToBP_Character (.HitActor (Collision|BreakHitResult _array_element)))
    (Variables|Default|SetBattle true)
    (return _returnvalue_2)))

(fn AttackRange
  (bind _returnvalue (Transformation|GetActorLocation))
  (Variables|Default|SetRange_Value 2e+01)
  (bind (_outhits _returnvalue_2) (Class|KismetSystemLibrary|BoxTraceMultiforObjects _returnvalue (+ _returnvalue (Math|Vector|MakeVector (* (Variables|Default|GetRotation) (Variables|Default|GetRange_Value)) 0.0 0.0)) (Math|Vector|MakeVector 16.0 5.0 2e+01) (Math|Rotator|MakeRotator (Variables|Default|GetRotation) 0.0 0.0) (Utilities|Array|MakeArray "ObjectTypeQuery3") false (Utilities|Array|MakeArray (Components|GetOwner)) "None" true "(R=1.000000,G=0.000000,B=0.000000,A=1.000000)" "(R=0.000000,G=1.000000,B=0.000000,A=1.000000)" 3.0))
  (for _array_element _outhits
    (Utilities|Casting|CastToBP_Character (.HitActor (Collision|BreakHitResult _array_element)))
    (return _returnvalue_2)))

(fn NewFunction
  (bind _asbp_character (Utilities|Casting|CastToBP_Character (Game|GetPlayerCharacter 0)))
  (if (and (or (Variables|/Game/New_Project/Blueprint/BP_Charater/BP_Character.BP_Character_C|GetDeath _asbp_character) (Variables|/Game/New_Project/Blueprint/BP_Charater/BP_Character.BP_Character_C|GetRolling _asbp_character)) (Utilities|Enum|NotEqual(Enum) (Variables|Default|GetMonster_State) "NewEnumerator3"))
    (Variables|Default|SetMonster_State "NewEnumerator0")))