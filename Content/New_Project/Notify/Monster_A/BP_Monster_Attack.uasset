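; Animation notify that makes BP_Monster_A fire a BP_Bullet at the player.
; On notify, it casts the owning actor to the monster and spawns the bullet at its PistolPoint.
; Aim follows the direction from monster to player character, with slight random spread on pitch only.
; The monster is set as the bullet's Owner, but the player character is set as its Instigator.
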(event EventOnReceiveNotify
  (params (OwningInstance :type Paper%20ZD%20Anim%20Instance%20Object%20Reference))
  (bind _returnvalue (Game|GetPlayerCharacter 0))
  (Utilities|IsValid OwningInstance
    (:Is%20Valid
      (bind _asbp_monster_a (Utilities|Casting|CastToBP_Monster_A (Class|PaperZDAnimInstance|GetOwningActor OwningInstance)))
      (Game|SpawnActorfromClass "/Game/New_Project/Blueprint/Monster_A/bullet/BP_Bullet.BP_Bullet_C" (Math|Transform|MakeTransform (Transformation|GetWorldLocation (Variables|/Game/New_Project/Blueprint/Monster_A/BP_Monster_A.BP_Monster_A_C|GetPistol_Point _asbp_monster_a)) (Math|Rotator|MakeRotator (.Roll (Math|Rotator|BreakRotator (Math|Conversions|RotationFromXVector (Math|Vector|GetUnitDirection(Vector) (Transformation|GetActorLocation _asbp_monster_a) (Transformation|GetActorLocation _returnvalue))))) (+ (.Pitch (Math|Rotator|BreakRotator (Math|Conversions|RotationFromXVector (Math|Vector|GetUnitDirection(Vector) (Transformation|GetActorLocation _asbp_monster_a) (Transformation|GetActorLocation _returnvalue))))) (Math|Random|RandomFloatinRange -3.0 3.0)) (.Yaw (Math|Rotator|BreakRotator (Math|Conversions|RotationFromXVector (Math|Vector|GetUnitDirection(Vector) (Transformation|GetActorLocation _asbp_monster_a) (Transformation|GetActorLocation _returnvalue)))))) "1.000000,1.000000,1.000000") "AlwaysSpawn" "MultiplyWithRoot" _asbp_monster_a _returnvalue))))